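; AI controller for the skeleton soldier that runs the BT_Soldier_AI behavior tree and feeds its blackboard with player detection.
; Sight of the first-person character sets the enemy actor and seen flag; losing sight starts a cooldown timer before the enemy is cleared.
; Heard noises, player collisions and damage set an investigate location, and damage also flags the soldier as hit.
; Perception tells sight from hearing by stimulus array index.
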(event `self.ReceivePossess`
  (params (PossessedPawn :type "Pawn Object Reference"))
  (add `self.OnTakeAnyDamage` PossessedPawn (delegate `OnTakeAnyDamage_Event`))
  (add `self.OnActorHit` PossessedPawn (delegate `OnHit_Event`))
  (`self.RunBehaviorTree` "/Game/Characters/Soldier/AI/BT_Soldier_AI.BT_Soldier_AI"))

(event `OnHit_Event` :!signature `self.OnActorHit`
  (params (SelfActor :type "Actor Object Reference") (OtherActor :type "Actor Object Reference") (NormalImpulse :type "Vector Structure") (Hit :type "HitResult Structure (by ref)"))
  (bind _asfirst_person_character (cast `/Game/Blueprints/Framework/FirstPersonCharacter` OtherActor))
  (`self.SetInvestigateTargetLocation` (`self.K2_GetActorLocation` _asfirst_person_character)))

(event `OnTakeAnyDamage_Event` :!signature `self.OnTakeAnyDamage`
  (params (DamagedActor :type "Actor Object Reference") (Damage :type "Float (double-precision)") (DamageType :type "DamageType Object Reference") (InstigatedBy :type "Controller Object Reference") (DamageCauser :type "Actor Object Reference"))
  (`self.SetInvestigateTargetLocation` (`self.K2_GetActorLocation` DamageCauser))
  (`self.SetIsHit`))

(event `self.AIPerception.OnPerceptionUpdated`
  (params (UpdatedActors :type "Array of Actor Object Reference (by ref)"))
  ;[1 1 1] Checking for Stimuli
  (for _array_element UpdatedActors
    (bind _info (`AIPerceptionComponent.GetActorsPerception` (`self.AIPerception`) _array_element))
    (cast `/Game/Blueprints/Framework/FirstPersonCharacter` _array_element)
    (for (_array_element_2 _array_index) (`.LastSensedStimuli` (break `ActorPerceptionBlueprintInfo` _info))
      (switch `int` _array_index
        (:`0`
          (bind (_age _expirationage _strength _stimuluslocation _receiverlocation _tag _bsuccessfullysensed) (break `AIStimulus` _array_element_2))
          ;[1 1 1] Sight Stimulus
          (if _bsuccessfullysensed
            (`KismetSystemLibrary.K2_ClearAndInvalidateTimerHandle` (`self.EnemyTimer`))
            (`BlackboardComponent.SetValueAsObject` (`self.Blackboard`) (`self.EnemyActorBBName`) _array_element)
            (`BlackboardComponent.SetValueAsBool` (`self.Blackboard`) (`self.IsEnemySeenBB`) true)
            (else
              (bind _returnvalue (`KismetSystemLibrary.K2_SetTimerDelegate` (delegate `StartEnemyTimer`) (`self.EnemyActorKeepCooldown`)))
              (set `self.EnemyTimer` _returnvalue)
              (`BlackboardComponent.SetValueAsBool` (`self.Blackboard`) (`self.IsEnemySeenBB`) false))))
        (:`1`
          ;[1 1 1] Hearing Stimulus
          (if _bsuccessfullysensed
            (`self.SetInvestigateTargetLocation` _stimuluslocation)))))))

(event `StartEnemyTimer`
  ;[1 1 1] Sight Stimulus
  (`BlackboardComponent.ClearValue` (`self.Blackboard`) (`self.EnemyActorBBName`)))

(fn `SetInvestigateTargetLocation`
  (params (TargetLocation :type "Vector Structure"))
  (`BlackboardComponent.SetValueAsVector` (`self.Blackboard`) (`self.InvestigateTargetLocationBBName`) TargetLocation)
  (return))

(fn `SetIsHit`
  (`BlackboardComponent.SetValueAsBool` (`self.Blackboard`) (`self.IsHitBBName`) true))

(fn `UserConstructionScript`)