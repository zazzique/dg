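; Base Blueprint for a button that the player presses by walking into its Box collision.
; An overlap from player character 0 is ignored while IsLocked is set; otherwise AutoLock can lock the button after that press.
; Each press fires OnPress, then toggles IsOn and fires OnSwitchOn or OnSwitchOff to announce the new state.
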(event `self.Box.OnComponentBeginOverlap`
  (params (OverlappedComponent :type "PrimitiveComponent Object Reference") (OtherActor :type "Actor Object Reference") (OtherComp :type "PrimitiveComponent Object Reference") (OtherBodyIndex :type Integer) (bFromSweep :type Boolean) (SweepResult :type "HitResult Structure (by ref)"))
  (if (and (== OtherActor (`GameplayStatics.GetPlayerCharacter` 0)) (not (`self.IsLocked`)))
    (`|ExecutionSequence`
      (:`then_0`
        (if (`self.AutoLock`)
          (set `self.IsLocked` true)))
      (:`then_1`
        (`self.OnPress`)
        (if (`self.IsOn`)
          (`self.OnSwitchOff`)
          (set `self.IsOn` false)
          (else
            (`self.OnSwitchOn`)
            (set `self.IsOn` true)))))))

(fn `UserConstructionScript`)