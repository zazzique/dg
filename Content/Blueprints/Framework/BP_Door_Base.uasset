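; BP_Door_Base is a base door Blueprint that can open and close automatically as the player approaches and leaves.
; When IsTriggerControlled is set, box collision overlaps by player character 0 invoke CallOpen on entry and CallClose on exit.
; OpenCloseInternal takes Open and Instant parameters but is empty here, as is the construction script, so this file defines no door motion.
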(event `self.Box Collision.OnComponentBeginOverlap`
  (params (OverlappedComponent :type "PrimitiveComponent Object Reference") (OtherActor :type "Actor Object Reference") (OtherComp :type "PrimitiveComponent Object Reference") (OtherBodyIndex :type Integer) (bFromSweep :type Boolean) (SweepResult :type "HitResult Structure (by ref)"))
  ;[1 1 1] Trigger Handling
  (if (and (== OtherActor (`GameplayStatics.GetPlayerCharacter` 0)) (`self.IsTriggerControlled`))
    (`self.Open`)))

(event `self.Box Collision.OnComponentEndOverlap`
  (params (OverlappedComponent :type "PrimitiveComponent Object Reference") (OtherActor :type "Actor Object Reference") (OtherComp :type "PrimitiveComponent Object Reference") (OtherBodyIndex :type Integer))
  ;[1 1 1] Trigger Handling
  (if (and (`self.IsTriggerControlled`) (== (`GameplayStatics.GetPlayerCharacter` 0) OtherActor))
    (`self.Close`)))

(fn `OpenCloseInternal`
  (params (Open :type Boolean) (Instant :type Boolean :default false)))

(fn `UserConstructionScript`)