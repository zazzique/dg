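; Base explosive actor that loses health from any non-melee damage and explodes when it reaches zero.
; AnyDamage feeds ExplodeInternal, where a once-only guard triggers radial damage and an explosion emitter at the bounds origin, then destroys the actor.
; The blast reuses the final hit's damage amount, credits its instigator and uses an explosion damage type, so it can chain to nearby explosives.
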(event `self.ReceiveAnyDamage`
  (params (Damage :type "Float (single-precision)") (DamageType :type "DamageType Object Reference") (InstigatedBy :type "Controller Object Reference") (DamageCauser :type "Actor Object Reference"))
  (`self.Explode Internal` Damage self InstigatedBy DamageType))

(fn `Explode Internal`
  (params (Damage :type "Float (double-precision)") (`Damage Causer` :type "Actor Object Reference") (`Damage Instigator` :type "Controller Object Reference") (DamageType :type "DamageType Object Reference"))
  (bind _origin (`self.GetActorBounds` false))
  (cast `DGDamageTypeMelee` DamageType
    (:`CastFailed`
      (bind _output_get (set `self.Health` (- (`self.Health`) Damage)))
      (if (<= _output_get 0.0)
        (`/Engine/EditorBlueprintResources/StandardMacros.DoOnce` (`self.IsExploded`)
          (:`Completed`
            (set `self.IsExploded` true)
            (`GameplayStatics.ApplyRadialDamage` (`self.Damage`) _origin (`self.Radius`) "/Script/DG.DGDamageTypeExplosion" (`|MakeArray` self :!type "Actor Object Reference") `Damage Causer` `Damage Instigator` false "ECC_GameTraceChannel2")
            (`GameplayStatics.SpawnEmitterAtLocation` "/Game/Particles/P_Explosion_01.P_Explosion_01" _origin)
            (`self.K2_DestroyActor`)))))))

(fn `UserConstructionScript`)