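; Base Blueprint for a breakable lamp with a point light that can switch on and off.
; BeginPlay sets the initial state from IsOnByDefault, and each state change swaps the mesh's light material slot and toggles PointLight visibility.
; Any damage breaks the lamp, applying the broken material, hiding the light and setting IsBroken, which blocks further switching.
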(event `self.ReceiveBeginPlay`
  (if (`self.IsOnByDefault`)
    (`self.Switch On`)
    (else
      (`self.SwitchOff`))))

(event `self.ReceiveAnyDamage`
  (params (Damage :type "Float (single-precision)") (DamageType :type "DamageType Object Reference") (InstigatedBy :type "Controller Object Reference") (DamageCauser :type "Actor Object Reference"))
  (`self.Break`))

(event `self.Break`
  (`PrimitiveComponent.SetMaterial` (`self.Mesh`) (`self.LightMaterialIndex`) "/Game/Blueprints/Lamps/SRC/M_Lamps_Set_1_Broken.M_Lamps_Set_1_Broken")
  (`SceneComponent.SetVisibility` (`self.PointLight`) false false)
  (set `self.IsBroken` true))

(event `self.Switch On`
  (if (not (`self.IsBroken`))
    (`PrimitiveComponent.SetMaterial` (`self.Mesh`) (`self.LightMaterialIndex`) "/Game/Blueprints/Lamps/SRC/M_Lamps_Set_1_On.M_Lamps_Set_1_On")
    (`SceneComponent.SetVisibility` (`self.PointLight`) true false)))

(event `self.SwitchOff`
  (if (not (`self.IsBroken`))
    (`PrimitiveComponent.SetMaterial` (`self.Mesh`) (`self.LightMaterialIndex`) "/Game/Blueprints/Lamps/SRC/M_Lamps_Set_1_Off.M_Lamps_Set_1_Off")
    (`SceneComponent.SetVisibility` (`self.PointLight`) false false)))

(fn `UserConstructionScript`)