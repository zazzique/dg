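; Door Blueprint variant (ES01, 6x4) that slides a single Door component between closed and open positions.
; On BeginPlay it binds open and close events and snaps to the open location if IsOpened is set.
; Opening plays the DoorLocation timeline to lerp the position unless IsLocked, while closing reverses that timeline without a lock check.
; OpenCloseInternal is empty.
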(event `self.ReceiveBeginPlay`
  (add `self.Open` (delegate `Open_Event`))
  (add `self.Close` (delegate `Close_Event`))
  (if (`self.IsOpened`)
    (`SceneComponent.K2_SetRelativeLocation` (`self.Door`) (`self.Open Location`) false false)))

(event `Open_Event`
  (if (not (`self.IsLocked`))
    (bind (_direction _location) (`Timeline|Door Location` :!label _label)
      (:`Update`
        (`SceneComponent.K2_SetRelativeLocation` (`self.Door`) (`KismetMathLibrary.VLerp` (`self.Close Location`) (`self.Open Location`) _location) false false)))))

(event `Close_Event`
  (goto _label :!via `Reverse`))

(fn `OpenCloseInternal`
  (params (Open :type Boolean) (Instant :type Boolean)))

(fn `UserConstructionScript`
  (`parent.UserConstructionScript`))